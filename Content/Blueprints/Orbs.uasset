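; Orb pickup for a side-scroller bird player that triggers a drug event with set intensity and duration, plus the bird's next thought and post-high music.
; Touching the Box removes the orb's light and collision box, fades current audio and starts the orb's high music.
; Nested-style WalkSlow and WalkSlower volumes cut walk speed until pickup, with WalkSlow also slowing the sprite.
; The float timeline is never triggered, and SetMusic ignores its StartTime.
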(event OnComponentBeginOverlap(Orb)
  (params (OverlappedComponent :type Primitive%20Component%20Object%20Reference) (OtherActor :type Actor%20Object%20Reference) (OtherComp :type Primitive%20Component%20Object%20Reference) (OtherBodyIndex :type Integer) (bFromSweep :type Boolean) (SweepResult :type Hit%20Result%20Structure%20%28by%20ref%29))
  ;[1 1 1] Code To Delete Orb
  (Actor|DestroyActor))

(event OnComponentBeginOverlap(Box)
  (params (OverlappedComponent :type Primitive%20Component%20Object%20Reference) (OtherActor :type Actor%20Object%20Reference) (OtherComp :type Primitive%20Component%20Object%20Reference) (OtherBodyIndex :type Integer) (bFromSweep :type Boolean) (SweepResult :type Hit%20Result%20Structure%20%28by%20ref%29))
  ;[1 1 1] Code To Delete Orb
  (if (Actor|ActorHasTag OtherActor "Player")
    (bind _as2dside_scroller_bird (Utilities|Casting|CastTo2DSideScrollerBird OtherActor))
    (Variables|/Game/2DSideScrollerBP/Blueprints/2DSideScrollerBird.2DSideScrollerBird_C|SetNextPostHigh _as2dside_scroller_bird (Variables|Default|GetPostHighMusic))
    (Variables|/Game/2DSideScrollerBP/Blueprints/2DSideScrollerBird.2DSideScrollerBird_C|SetNextThought _as2dside_scroller_bird (Variables|Default|GetBirdThought))
    (Default|DrugEvent _as2dside_scroller_bird (Variables|Default|GetDrugIntensity) (Variables|Default|GetDrugDuration))
    (Components|DestroyComponent (Variables|Default|GetPointLight))
    (Components|DestroyComponent (Variables|Default|GetOrb))
    (Components|DestroyComponent (Variables|Default|GetBox))
    (Variables|Default|SetcanEnter false)
    (Audio|Components|Audio|FadeOut (Variables|Default|GetSource) 1.0 0.0 :!class /Script/Engine.AudioComponent)
    (Audio|Components|Audio|FadeOut (Variables|/Game/MusicControl.MusicControl_C|GetMusicSource (Variables|Default|GetMusicObject)) 1.0 0.0 :!class /Script/Engine.AudioComponent)
    (CallFunction|SetMusic true (Variables|Default|GetOrbHighMusic) (Math|Random|RandomFloatinRange 0.0 16.0))))

(event OnComponentBeginOverlap(WalkSlow)
  (params (OverlappedComponent :type Primitive%20Component%20Object%20Reference) (OtherActor :type Actor%20Object%20Reference) (OtherComp :type Primitive%20Component%20Object%20Reference) (OtherBodyIndex :type Integer) (bFromSweep :type Boolean) (SweepResult :type Hit%20Result%20Structure%20%28by%20ref%29))
  ;[1 1 1] Player Speed Editing
  (if (and (Actor|ActorHasTag OtherActor "Player") (Variables|Default|GetcanEnter))
    (bind _as2dside_scroller_bird (Utilities|Casting|CastTo2DSideScrollerBird OtherActor))
    (Variables|Default|SetsavedSpeed (Variables|/Script/Engine.CharacterMovementComponent|GetMaxWalkSpeed (Variables|/Script/Engine.Character|GetCharacterMovement _as2dside_scroller_bird)))
    (Variables|/Script/Engine.CharacterMovementComponent|SetMaxWalkSpeed (Variables|/Script/Engine.Character|GetCharacterMovement _as2dside_scroller_bird) (/ (Variables|/Script/Engine.CharacterMovementComponent|GetMaxWalkSpeed (Variables|/Script/Engine.Character|GetCharacterMovement _as2dside_scroller_bird)) 2.0))
    (Components|Timeline|SetPlayRate (Variables|/Script/Paper2D.PaperCharacter|GetSprite _as2dside_scroller_bird) 0.5)))

(event OnComponentEndOverlap(WalkSlow)
  (params (OverlappedComponent :type Primitive%20Component%20Object%20Reference) (OtherActor :type Actor%20Object%20Reference) (OtherComp :type Primitive%20Component%20Object%20Reference) (OtherBodyIndex :type Integer))
  ;[1 1 1] Player Speed Editing
  (Development|PrintString "")
  (if (Actor|ActorHasTag OtherActor "Player")
    (bind _as2dside_scroller_bird (Utilities|Casting|CastTo2DSideScrollerBird OtherActor))
    (Variables|/Script/Engine.CharacterMovementComponent|SetMaxWalkSpeed (Variables|/Script/Engine.Character|GetCharacterMovement _as2dside_scroller_bird) (Variables|Default|GetsavedSpeed))
    (Components|Timeline|SetPlayRate (Variables|/Script/Paper2D.PaperCharacter|GetSprite _as2dside_scroller_bird) 1.0)))

(event OnComponentBeginOverlap(WalkSlower)
  (params (OverlappedComponent :type Primitive%20Component%20Object%20Reference) (OtherActor :type Actor%20Object%20Reference) (OtherComp :type Primitive%20Component%20Object%20Reference) (OtherBodyIndex :type Integer) (bFromSweep :type Boolean) (SweepResult :type Hit%20Result%20Structure%20%28by%20ref%29))
  ;[1 1 1] Player Speed Editing
  (if (and (Actor|ActorHasTag OtherActor "Player") (Variables|Default|GetcanEnter))
    (bind _as2dside_scroller_bird (Utilities|Casting|CastTo2DSideScrollerBird OtherActor))
    (Variables|/Script/Engine.CharacterMovementComponent|SetMaxWalkSpeed (Variables|/Script/Engine.Character|GetCharacterMovement _as2dside_scroller_bird) (/ (Variables|/Script/Engine.CharacterMovementComponent|GetMaxWalkSpeed (Variables|/Script/Engine.Character|GetCharacterMovement _as2dside_scroller_bird)) 2.0))))

(event OnComponentEndOverlap(WalkSlower)
  (params (OverlappedComponent :type Primitive%20Component%20Object%20Reference) (OtherActor :type Actor%20Object%20Reference) (OtherComp :type Primitive%20Component%20Object%20Reference) (OtherBodyIndex :type Integer))
  ;[1 1 1] Player Speed Editing
  (if (Actor|ActorHasTag "Player")
    (bind _as2dside_scroller_bird (Utilities|Casting|CastTo2DSideScrollerBird OtherActor))
    (Variables|/Script/Engine.CharacterMovementComponent|SetMaxWalkSpeed (Variables|/Script/Engine.Character|GetCharacterMovement _as2dside_scroller_bird) (/ (Variables|Default|GetsavedSpeed) 1.5))))

(event EventBeginPlay
  ;[1 1 1] FloatAnimation
)

(event Collision|EventActorBeginOverlap
  (params (OtherActor :type Actor%20Object%20Reference)))

(event EventTick
  (params (DeltaSeconds :type Float%20%28single-precision%29)))

(fn ConstructionScript)

(fn SetMusic
  (params (StartOnSet :type Boolean) (CueInput :type Sound%20Cue%20Object%20Reference) (StartTime :type Float%20%28single-precision%29))
  (Audio|Components|Audio|SetSound (Variables|/Game/MusicControl.MusicControl_C|GetMusicSource (Variables|Default|GetMusicObject)) CueInput)
  (if StartOnSet
    (Audio|Components|Audio|Play (Variables|/Game/MusicControl.MusicControl_C|GetMusicSource (Variables|Default|GetMusicObject)) 0.0)))

(fn ResetWalkSpeed
  (params (Character :type 2D%20Side%20Scroller%20Bird%20Object%20Reference))
  (Variables|/Script/Engine.CharacterMovementComponent|SetMaxWalkSpeed (Variables|/Script/Engine.Character|GetCharacterMovement Character) (Variables|Default|GetsavedSpeed)))