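; Goose Paper2D actor that stages the exit cutscene leading into the FinalAct level.
; WalkLeftEvent runs a timeline that lerps the goose in X toward a point just left of the player while CanWalk is set.
; When the player bird overlaps Box, it loses its sprite and the goose switches flipbook, mirrors via negative X scale and moves right on Tick.
; A delayed camera fade then precedes the level load.
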(event OnComponentBeginOverlap(Box)
  (params (OverlappedComponent :type Primitive%20Component%20Object%20Reference) (OtherActor :type Actor%20Object%20Reference) (OtherComp :type Primitive%20Component%20Object%20Reference) (OtherBodyIndex :type Integer) (bFromSweep :type Boolean) (SweepResult :type Hit%20Result%20Structure%20%28by%20ref%29))
  (bind _returnvalue (Transformation|GetActorScale3D))
  (bind (_x _y _z) (Math|Vector|BreakVector _returnvalue))
  ;[1 1 1] Preps level load for final level
  (if (Actor|ActorHasTag OtherActor "Player")
    (bind _as2dside_scroller_bird (Utilities|Casting|CastTo2DSideScrollerBird OtherActor))
    (Default|DestroySprite _as2dside_scroller_bird)
    (Components|DestroyComponent (Variables|Default|GetBox))
    (Variables|Default|SetcanWalk false)
    (Development|PrintString "")
    (Sprite|SetFlipbook (Variables|Default|GetRenderComponent) "/Game/SexyBoy/GooseAndSparrow/GNSWalk.GNSWalk")
    (Transformation|SetActorScale3D (Math|Vector|MakeVector (* _x -1.0) _y _z))
    (Utilities|FlowControl|Delay 1.0)
    (Variables|Default|SetwalkRight true)
    (Utilities|FlowControl|Delay 3.0)
    (CameraFades|StartCameraFade :self (Game|GetPlayerCameraManager 0) :ToAlpha 1.0 :Duration 2.0 :bHoldWhenFinished true)
    (Utilities|FlowControl|Delay 3.0)
    (Game|OpenLevel(byName) "FinalAct")))

(event Custom|WalkLeftEvent
  (bind _returnvalue (Transformation|GetActorLocation))
  (bind (_x _y _z) (Math|Vector|BreakVector _returnvalue))
  ;[1 1 1] Goose's inital movement
  (bind _righttoleft (Timeline|WalkTimeline PlayFromStart)
    (:Update
      (if (Variables|Default|GetcanWalk)
        (Transformation|SetActorLocation (Math|Vector|Lerp(Vector) _returnvalue (Math|Vector|MakeVector (- (.X (Math|Vector|BreakVector (Transformation|GetActorLocation (Variables|Default|GetPlayerActor)))) 1e+02) _y _z) _righttoleft) false false)))))

(event EventTick
  (params (DeltaSeconds :type Float%20%28single-precision%29))
  ;[1 1 1] Goose's exit animations
  (if (Variables|Default|GetwalkRight)
    (Transformation|SetActorLocation (+ (Transformation|GetActorLocation) (Math|Vector|MakeVector (/ (Variables|Default|GetSpeed) 1e+01) 0.0 0.0)) false false)))

(fn ConstructionScript)